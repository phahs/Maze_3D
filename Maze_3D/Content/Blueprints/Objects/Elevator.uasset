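; Elevator actor that shuttles a platform back and forth, with a randomized starting direction and initial wait.
; Tick accumulates a timer until it reaches WaitFor, then a DoOnce plays the MoveElevator timeline forward or in reverse, depending on AtTop.
; The timeline offsets the elevator from its starting position, then flips direction and resets the wait on finishing.
; RotateElevatorto turns the tile in quarter steps according to an existing-wall index.
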(event `self.ReceiveBeginPlay`
  (set `self.AtTop` (`KismetMathLibrary.RandomBool`))
  (set `self.StartPosition` (`SceneComponent.K2_GetComponentLocation` (`self.Elevator Tile`)))
  (set `self.Timer` (`KismetMathLibrary.RandomFloatInRange` 0.0 5.0)))

(event `self.ReceiveTick`
  (params (DeltaSeconds :type "Float (single-precision)"))
  (bind _timer (`self.Timer`))
  (if (<= (`self.WaitFor`) _timer)
    (`/Engine/EditorBlueprintResources/StandardMacros.DoOnce` false :!label _label
      (:`Completed`
        (if (`self.AtTop`)
          (bind (_direction _oscillate) (`Timeline|MoveElevator` :!via `ReverseFromEnd` :!label _label_2)
            (:`Update`
              (`SceneComponent.K2_SetWorldLocation` (`self.Elevator`) (+ (`self.StartPosition`) _oscillate) false false))
            (:`Finished`
              (set `self.AtTop` (not (`self.AtTop`)))
              (set `self.Timer` 0.0)
              (goto _label :!via `Reset`)))
          (else
            (goto _label_2 :!via `PlayFromStart`)))))
    (else
      (set `self.Timer` (+ _timer DeltaSeconds)))))

(event `self.RotateElevatorTo`
  (params (existingWall :type Integer))
  (bind _elevator_tile (`self.Elevator Tile`))
  (switch `int` existingWall
    (:`1`
      (`SceneComponent.K2_SetWorldRotation` _elevator_tile (struct :`Yaw` 180.0) false false))
    (:`2`
      (`SceneComponent.K2_SetWorldRotation` _elevator_tile (struct :`Yaw` 270.0) false false))
    (:`3`
      (`SceneComponent.K2_SetWorldRotation` :`self` _elevator_tile))
    (:`4`
      (`SceneComponent.K2_SetWorldRotation` _elevator_tile (struct :`Yaw` 90.0) false false))))

(fn `UserConstructionScript`)