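; Exit room actor for the 3D maze that labels itself with exit, continue and level text.
; On BeginPlay it casts the widgets behind its ExitText, ContinueText and MazeLevelText components to the Text widget and sets their strings.
; The maze level comes from Maze_3D_GameMode; from level 50 onward the labels switch to a final-level message and a replay prompt.
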(event `self.ReceiveBeginPlay`
  (bind _astext (cast `/Game/Blueprints/UI/Text` (`WidgetComponent.GetUserWidgetObject` (`self.Exit Text`))))
  (set `/Game/Blueprints/UI/Text.What to say` "Exit" _astext)
  (bind _astext_2 (cast `/Game/Blueprints/UI/Text` (`WidgetComponent.GetUserWidgetObject` (`self.Continue Text`))))
  (set `/Game/Blueprints/UI/Text.What to say` "Continue?" _astext_2)
  (bind _asmaze_3d_game_mode (cast `Maze_3D_GameMode` (`GameplayStatics.GetGameMode`)))
  (bind _returnvalue (`Maze_3D_GameMode.GetMazeLevel` _asmaze_3d_game_mode))
  (if (< _returnvalue 50)
    (bind _astext_3 (cast `/Game/Blueprints/UI/Text` (`WidgetComponent.GetUserWidgetObject` (`self.MazeLevel Text`))))
    (set `/Game/Blueprints/UI/Text.What to say` (`KismetTextLibrary.Conv_StringToText` (`KismetStringLibrary.Concat_StrStr` "Level: " (`KismetStringLibrary.Conv_IntToString` _returnvalue))) _astext_3)
    (else
      (bind _astext_4 (cast `/Game/Blueprints/UI/Text` (`WidgetComponent.GetUserWidgetObject` (`self.MazeLevel Text`))))
      (set `/Game/Blueprints/UI/Text.What to say` (`KismetTextLibrary.Conv_StringToText` "Final Level!") _astext_4)
      (bind _astext_5 (cast `/Game/Blueprints/UI/Text` (`WidgetComponent.GetUserWidgetObject` (`self.Continue Text`))))
      (set `/Game/Blueprints/UI/Text.What to say` "Replay Last Level?" _astext_5))))

(fn `UserConstructionScript`)