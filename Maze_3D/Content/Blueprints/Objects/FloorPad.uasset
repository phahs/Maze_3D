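; FloorPad is a maze trigger pad, colored red when IsExit is set and green otherwise.
; When MazePlayer_BP overlaps its capsule, it calls UpdateLevel on Maze_3D_GameMode.
; An exit pad then writes the game instance's level and size to a save slot and opens MainMenu on success.
; A non-exit pad instead calls ExitFound on the game mode.
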(event `self.ReceiveBeginPlay`
  (bind _cylinder (`self.Cylinder`))
  (bind _asmaze_3d_game_mode (cast `Maze_3D_GameMode` (`GameplayStatics.GetGameMode`)))
  (bind _returnvalue (`Maze_3D_GameMode.GetMazeLevel` _asmaze_3d_game_mode))
  (set `self.Level` _returnvalue)
  (bind _returnvalue_2 (`Maze_3D_GameMode.GetMazeSize` _asmaze_3d_game_mode))
  (set `self.Size` _returnvalue_2)
  (if (`self.isExit`)
    (`PrimitiveComponent.SetMaterial` _cylinder 0 "/Game/Materials/Color_Red.Color_Red")
    (else
      (`PrimitiveComponent.SetMaterial` _cylinder 0 "/Game/Materials/Color_Green.Color_Green"))))

(event `self.Capsule.OnComponentBeginOverlap`
  (params (OverlappedComponent :type "PrimitiveComponent Object Reference") (OtherActor :type "Actor Object Reference") (OtherComp :type "PrimitiveComponent Object Reference") (OtherBodyIndex :type Integer) (bFromSweep :type Boolean) (SweepResult :type "HitResult Structure (by ref)"))
  (`/Engine/EditorBlueprintResources/StandardMacros.IsValid` OtherActor
    (:`Is Valid`
      (cast `/Game/Blueprints/Player/MazePlayer_BP` OtherActor)
      (bind _asmaze_3d_game_mode (cast `Maze_3D_GameMode` (`GameplayStatics.GetGameMode`)))
      (`Maze_3D_GameMode.UpdateLevel` _asmaze_3d_game_mode)
      (if (`self.isExit`)
        (bind _returnvalue (`GameplayStatics.CreateSaveGameObject` "/Game/Blueprints/MazeSaveGameBP.MazeSaveGameBP_C"))
        (bind _asmaze_3d_game_instance (cast `Maze_3D_GameInstance` (`GameplayStatics.GetGameInstance`)))
        (bind (_level _size) (`Maze_3D_GameInstance.SendLevelInfo` _asmaze_3d_game_instance))
        (`MazeSaveGame.SetLevel` _returnvalue _level)
        (`MazeSaveGame.SetSize` _returnvalue _size)
        (bind _returnvalue_2 (`GameplayStatics.SaveGameToSlot` _returnvalue "Maze_3D_Save"))
        (if _returnvalue_2
          (`GameplayStatics.OpenLevel` "MainMenu"))
        (else
          (`Maze_3D_GameMode.ExitFound` _asmaze_3d_game_mode))))))

(fn `UserConstructionScript`)