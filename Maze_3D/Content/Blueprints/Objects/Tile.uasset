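; Tile actor for a modular level cell with a floor, four walls and a ceiling that can be opened by direction.
; RemoveWall calls the parent version, then hides the chosen piece and disables its collision; the ceiling case also covers its child CielingLight actor.
; MakeExitRoom spawns an Exit_RoomBP beside the tile on the given horizontal side, offset and rotated to match that direction.
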(event `self.ReceiveBeginPlay`)

(event `self.RemoveWall`
  (params (dir :type Integer))
  (bind _floor (`self.Floor`))
  (bind _frontwall (`self.FrontWall`))
  (bind _rightwall (`self.RightWall`))
  (bind _backwall (`self.BackWall`))
  (bind _leftwall (`self.LeftWall`))
  (bind _cieling (`self.Cieling`))
  (`parent.RemoveWall` dir)
  (switch `int` dir
    (:`0`
      (`SceneComponent.SetHiddenInGame` _floor true false)
      (`PrimitiveComponent.SetCollisionEnabled` _floor "NoCollision"))
    (:`1`
      (`SceneComponent.SetHiddenInGame` _frontwall true false)
      (`PrimitiveComponent.SetCollisionEnabled` _frontwall "NoCollision"))
    (:`2`
      (`SceneComponent.SetHiddenInGame` _rightwall true false)
      (`PrimitiveComponent.SetCollisionEnabled` _rightwall "NoCollision"))
    (:`3`
      (`SceneComponent.SetHiddenInGame` _backwall true false)
      (`PrimitiveComponent.SetCollisionEnabled` _backwall "NoCollision"))
    (:`4`
      (`SceneComponent.SetHiddenInGame` _leftwall true false)
      (`PrimitiveComponent.SetCollisionEnabled` _leftwall "NoCollision"))
    (:`5`
      (`SceneComponent.SetHiddenInGame` _cieling true true)
      (bind _ascieling_light (cast `/Game/Blueprints/Objects/CielingLight` (`ChildActorComponent.ChildActor` (`self.ChildActor`))))
      (`PrimitiveComponent.SetCollisionEnabled` _cieling "NoCollision")
      (`PrimitiveComponent.SetCollisionEnabled` (`/Game/Blueprints/Objects/CielingLight.Cylinder` _ascieling_light) "NoCollision")
      (`PrimitiveComponent.SetCollisionEnabled` (`/Game/Blueprints/Objects/CielingLight.Sphere` _ascieling_light) "NoCollision"))))

(event `self.MakeExitRoom`
  (params (ExitDirection :type Integer))
  (bind _location (.location (`self.GetTransform` self)))
  (switch `int` ExitDirection
    (:`1`
      (set `self.Loc` (+ _location (0.0 149.0 0.0)))
      (set `self.Rot` (struct :`Yaw` 180.0)))
    (:`2`
      (set `self.Loc` (+ _location (-149.0 0.0 0.0)))
      (set `self.Rot` (struct :`Yaw` 270.0)))
    (:`3`
      (set `self.Loc` (+ _location (0.0 -149.0 0.0)))
      (set `self.Rot` (struct)))
    (:`4`
      (set `self.Loc` (+ _location (149.0 0.0 0.0)))
      (set `self.Rot` (struct :`Yaw` 90.0))))
  (`|SpawnActorFromClass` "/Game/Blueprints/Objects/Exit_RoomBP.Exit_RoomBP_C" (`KismetMathLibrary.MakeTransform` (`self.Loc`) (`self.Rot`)) "Undefined" "OverrideRootScale" null null))

(fn `UserConstructionScript`)